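; DS_Camera is an input-binding Blueprint for a camera, handling six-direction movement and increment/decrement of a value.
; Each Enhanced Input action routes Triggered, Started and Ongoing to a Started handler, and Canceled and Completed to a Completed handler.
; Movement handlers receive the action value repackaged as an Axis1D input value; increment and decrement handlers take none.
; The handler logic lives outside these graphs, and the construction script is empty.
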(event Input|EnhancedActionEvents|EnhancedInputActionDS_MoveForward
  (params (ActionValue :type Float%20%28double-precision%29) (ElapsedSeconds :type Float%20%28double-precision%29) (TriggeredSeconds :type Float%20%28double-precision%29) (InputAction :type Input%20Action%20Object%20Reference :default "/DS_CameraSuite/Inputs/Actions/DS_MoveForward.DS_MoveForward"))
  (bind _returnvalue (Class|EnhancedInputLibrary|MakeInputActionValueOfType ActionValue ActionValue ActionValue "Axis1D"))
  ;[1 1 1] DS - Enhanced Input Components
  (:Triggered
    (Class|DSCamera|MoveForwardStarted _returnvalue :!label _label))
  (:Started
    (goto _label))
  (:Ongoing
    (goto _label))
  (:Canceled
    (Class|DSCamera|MoveForwardCompleted _returnvalue :!label _label_2))
  (:Completed
    (goto _label_2)))

(event Input|EnhancedActionEvents|EnhancedInputActionDS_MoveBackwards
  (params (ActionValue :type Float%20%28double-precision%29) (ElapsedSeconds :type Float%20%28double-precision%29) (TriggeredSeconds :type Float%20%28double-precision%29) (InputAction :type Input%20Action%20Object%20Reference :default "/DS_CameraSuite/Inputs/Actions/DS_MoveBackwards.DS_MoveBackwards"))
  (bind _returnvalue (Class|EnhancedInputLibrary|MakeInputActionValueOfType ActionValue ActionValue ActionValue "Axis1D"))
  ;[1 1 1] DS - Enhanced Input Components
  (:Triggered
    (Class|DSCamera|MoveBackwardStarted _returnvalue :!label _label))
  (:Started
    (goto _label))
  (:Ongoing
    (goto _label))
  (:Canceled
    (Class|DSCamera|MoveBackwardCompleted _returnvalue :!label _label_2))
  (:Completed
    (goto _label_2)))

(event Input|EnhancedActionEvents|EnhancedInputActionDS_MoveLeft
  (params (ActionValue :type Float%20%28double-precision%29) (ElapsedSeconds :type Float%20%28double-precision%29) (TriggeredSeconds :type Float%20%28double-precision%29) (InputAction :type Input%20Action%20Object%20Reference :default "/DS_CameraSuite/Inputs/Actions/DS_MoveLeft.DS_MoveLeft"))
  (bind _returnvalue (Class|EnhancedInputLibrary|MakeInputActionValueOfType ActionValue ActionValue ActionValue "Axis1D"))
  ;[1 1 1] DS - Enhanced Input Components
  (:Triggered
    (Class|DSCamera|MoveLeftStarted _returnvalue :!label _label))
  (:Started
    (goto _label))
  (:Ongoing
    (goto _label))
  (:Canceled
    (Class|DSCamera|MoveLeftCompleted _returnvalue :!label _label_2))
  (:Completed
    (goto _label_2)))

(event Input|EnhancedActionEvents|EnhancedInputActionDS_MoveRight
  (params (ActionValue :type Float%20%28double-precision%29) (ElapsedSeconds :type Float%20%28double-precision%29) (TriggeredSeconds :type Float%20%28double-precision%29) (InputAction :type Input%20Action%20Object%20Reference :default "/DS_CameraSuite/Inputs/Actions/DS_MoveRight.DS_MoveRight"))
  (bind _returnvalue (Class|EnhancedInputLibrary|MakeInputActionValueOfType ActionValue ActionValue ActionValue "Axis1D"))
  ;[1 1 1] DS - Enhanced Input Components
  (:Triggered
    (Class|DSCamera|MoveRightStarted _returnvalue :!label _label))
  (:Started
    (goto _label))
  (:Ongoing
    (goto _label))
  (:Canceled
    (Class|DSCamera|MoveRightCompleted _returnvalue :!label _label_2))
  (:Completed
    (goto _label_2)))

(event Input|EnhancedActionEvents|EnhancedInputActionDS_MoveUp
  (params (ActionValue :type Float%20%28double-precision%29) (ElapsedSeconds :type Float%20%28double-precision%29) (TriggeredSeconds :type Float%20%28double-precision%29) (InputAction :type Input%20Action%20Object%20Reference :default "/DS_CameraSuite/Inputs/Actions/DS_MoveUp.DS_MoveUp"))
  (bind _returnvalue (Class|EnhancedInputLibrary|MakeInputActionValueOfType ActionValue ActionValue ActionValue "Axis1D"))
  ;[1 1 1] DS - Enhanced Input Components
  (:Triggered
    (Class|DSCamera|MoveUpStarted _returnvalue :!label _label))
  (:Started
    (goto _label))
  (:Ongoing
    (goto _label))
  (:Canceled
    (Class|DSCamera|MoveUpCompleted _returnvalue :!label _label_2))
  (:Completed
    (goto _label_2)))

(event Input|EnhancedActionEvents|EnhancedInputActionDS_MoveDown
  (params (ActionValue :type Float%20%28double-precision%29) (ElapsedSeconds :type Float%20%28double-precision%29) (TriggeredSeconds :type Float%20%28double-precision%29) (InputAction :type Input%20Action%20Object%20Reference :default "/DS_CameraSuite/Inputs/Actions/DS_MoveDown.DS_MoveDown"))
  (bind _returnvalue (Class|EnhancedInputLibrary|MakeInputActionValueOfType ActionValue ActionValue ActionValue "Axis1D"))
  ;[1 1 1] DS - Enhanced Input Components
  (:Triggered
    (Class|DSCamera|MoveDownStarted _returnvalue :!label _label))
  (:Started
    (goto _label))
  (:Ongoing
    (goto _label))
  (:Canceled
    (Class|DSCamera|MoveDownCompleted _returnvalue :!label _label_2))
  (:Completed
    (goto _label_2)))

(event Input|EnhancedActionEvents|EnhancedInputActionDS_IncrementValue
  (params (ActionValue :type Float%20%28double-precision%29) (ElapsedSeconds :type Float%20%28double-precision%29) (TriggeredSeconds :type Float%20%28double-precision%29) (InputAction :type Input%20Action%20Object%20Reference :default "/DS_CameraSuite/Inputs/Actions/DS_IncrementValue.DS_IncrementValue"))
  ;[1 1 1] DS - Enhanced Input Components
  (:Triggered
    (Class|DSCamera|IncrementValueStarted :!label _label))
  (:Started
    (goto _label))
  (:Ongoing
    (goto _label))
  (:Canceled
    (Class|DSCamera|IncrementValueCompleted :!label _label_2))
  (:Completed
    (goto _label_2)))

(event Input|EnhancedActionEvents|EnhancedInputActionDS_DecrementValue
  (params (ActionValue :type Float%20%28double-precision%29) (ElapsedSeconds :type Float%20%28double-precision%29) (TriggeredSeconds :type Float%20%28double-precision%29) (InputAction :type Input%20Action%20Object%20Reference :default "/DS_CameraSuite/Inputs/Actions/DS_DecrementValue.DS_DecrementValue"))
  ;[1 1 1] DS - Enhanced Input Components
  (:Triggered
    (Class|DSCamera|DecrementValueStarted :!label _label))
  (:Started
    (goto _label))
  (:Ongoing
    (goto _label))
  (:Canceled
    (Class|DSCamera|DecrementValueCompleted :!label _label_2))
  (:Completed
    (goto _label_2)))

(fn ConstructionScript)